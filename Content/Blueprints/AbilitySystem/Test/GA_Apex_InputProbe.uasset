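; GA_Apex_InputProbe is a test gameplay ability that reports when it activates and on which network side.
; On activation it reads the display name from its skill definition, then prints it prefixed with Server or Client based on an authority check.
; It ends itself immediately afterward, with no other gameplay effect.
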(event Ability|EventActivateAbility
  (Variables|Default|SetDisplayName (Utilities|GetDisplayName (Class|ApexGameplayAbility|GetSkillDefinition)))
  (Ability|HasAuthority
    (:True
      (Development|PrintText (Utilities|Text|FormatText "Server {Name}" (Variables|Default|GetDisplayName))))
    (:False
      (Development|PrintText (Utilities|Text|FormatText "Client {Name}" (Variables|Default|GetDisplayName)))))
  (Ability|EndAbility))

(event Ability|EventOnEndAbility
  (params (bWasCancelled :type Boolean)))